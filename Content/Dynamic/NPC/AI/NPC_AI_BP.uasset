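; AI controller for guard NPCs that perceives targets and drives the guard's aiming and shooting.
; On BeginPlay it sets up the PatrolData blackboard and runs the GuardBehaviour behavior tree.
; Perception updates store sensed actors lacking the "Enemy" tag under EnemyKey, clearing it when sensing is lost.
; Each tick it sets the controlled GuardActor's Aiming and Shooting flags based on whether a focus actor exists.
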(event OnTargetPerceptionUpdated(AIPerception)
  (params (Actor :type Actor%20Object%20Reference) (Stimulus :type AI%20Stimulus%20Structure))
  (bind _blackboardcomponent (Variables|Default|GetBlackBoardComponent))
  (bind _enemykey (Variables|Default|GetEnemyKey))
  (if (not (Actor|ActorHasTag Actor "Enemy"))
    (bind _output_get (Variables|Default|SetSensed (.bSuccessfullySensed (Utilities|Struct|BreakAIStimulus Stimulus))))
    (if _output_get
      (AI|Components|Blackboard|SetValueasObject _blackboardcomponent _enemykey Actor)
      (else
        (AI|Components|Blackboard|ClearValue _blackboardcomponent _enemykey)))))

(event EventBeginPlay
  (bind _blackboardcomponent (Class|AIController|UseBlackboard "/Game/Dynamic/NPC/AI/PatrolData.PatrolData"))
  (Variables|Default|SetBlackBoardComponent _blackboardcomponent)
  (AI|RunBehaviorTree "/Game/Dynamic/NPC/AI/GuardBehaviour.GuardBehaviour"))

(event EventTick
  (params (DeltaSeconds :type Float%20%28single-precision%29))
  (bind _asguard_actor (Utilities|Casting|CastToGuardActor (Pawn|GetControlledPawn)))
  (bind _output_get (Variables|/Game/Dynamic/NPC/Behaviour/GuardActor.GuardActor_C|SetAiming _asguard_actor (Utilities|IsValid (Class|AIController|GetFocusActor))))
  (Variables|/Game/Dynamic/NPC/Behaviour/GuardActor.GuardActor_C|SetShooting _asguard_actor _output_get))

(fn ConstructionScript)