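; BP_AI is an AI controller for guard characters that detects targets through AI perception.
; On BeginPlay it sets up the PatrolData blackboard and runs the GuardBehaviour behavior tree.
; Perception updates for actors without the "Enemy" tag write the sensed actor to EnemyKey, or clear the key when sensing is lost.
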(event OnTargetPerceptionUpdated(AIPerception)
  (params (Actor :type Actor%20Object%20Reference) (Stimulus :type AI%20Stimulus%20Structure))
  (bind _blackboardcomponent (Variables|Default|GetBlackBoardComponent))
  (bind _enemykey (Variables|Default|GetEnemyKey))
  (if (not (Actor|ActorHasTag Actor "Enemy"))
    (bind _output_get (Variables|Default|SetSensed (.bSuccessfullySensed (Utilities|Struct|BreakAIStimulus Stimulus))))
    (if _output_get
      (AI|Components|Blackboard|SetValueasObject _blackboardcomponent _enemykey Actor)
      (else
        (AI|Components|Blackboard|ClearValue _blackboardcomponent _enemykey)))))

(event EventBeginPlay
  (bind _blackboardcomponent (Class|AIController|UseBlackboard "/Game/Dynamic/Character/AI/PatrolData.PatrolData"))
  (Variables|Default|SetBlackBoardComponent _blackboardcomponent)
  (AI|RunBehaviorTree "/Game/Dynamic/Character/AI/GuardBehaviour.GuardBehaviour"))

(fn ConstructionScript)