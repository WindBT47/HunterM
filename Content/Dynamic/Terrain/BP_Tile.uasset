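; BP_Tile is a terrain tile for an infinite terrain game, with a barrier that opens and closes around the player.
; When the player enters LockingValume, the barrier loses collision, turns green, and InfiniteTerrainGameMode spawns a tile.
; Leaving that volume restores collision and the red material, while entering DestroyVolume destroys the tile.
; GetAttachLocation exposes the Arrow component's world transform as an attach point.
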(event OnComponentBeginOverlap(LockingValume)
  (params (OverlappedComponent :type Primitive%20Component%20Object%20Reference) (OtherActor :type Actor%20Object%20Reference) (OtherComp :type Primitive%20Component%20Object%20Reference) (OtherBodyIndex :type Integer) (bFromSweep :type Boolean) (SweepResult :type Hit%20Result%20Structure%20%28by%20ref%29))
  (Utilities|IsPlayerActor OtherActor)
  (CallFunction|UnLock)
  (bind _asinfinite_terrain_game_mode (Utilities|Casting|CastToInfiniteTerrainGameMode (Game|GetGameMode)))
  (Default|SpawnTile _asinfinite_terrain_game_mode))

(event OnComponentEndOverlap(LockingValume)
  (params (OverlappedComponent :type Primitive%20Component%20Object%20Reference) (OtherActor :type Actor%20Object%20Reference) (OtherComp :type Primitive%20Component%20Object%20Reference) (OtherBodyIndex :type Integer))
  (Utilities|IsPlayerActor OtherActor)
  (CallFunction|Lock))

(event OnComponentBeginOverlap(DestroyVolume)
  (params (OverlappedComponent :type Primitive%20Component%20Object%20Reference) (OtherActor :type Actor%20Object%20Reference) (OtherComp :type Primitive%20Component%20Object%20Reference) (OtherBodyIndex :type Integer) (bFromSweep :type Boolean) (SweepResult :type Hit%20Result%20Structure%20%28by%20ref%29))
  (Utilities|IsPlayerActor OtherActor)
  (Actor|DestroyActor))

(fn ConstructionScript)

(fn GetAttachLocation
  (return (Transformation|GetWorldTransform (Variables|Default|GetArrow))))

(fn UnLock
  (bind _barrier (Variables|Default|GetBarrier))
  (Collision|SetCollisionEnabled _barrier "NoCollision")
  (Rendering|Material|SetMaterial _barrier 0 "/Game/Dynamic/Terrain/Green_Barrier.Green_Barrier"))

(fn Lock
  (bind _barrier (Variables|Default|GetBarrier))
  (Collision|SetCollisionEnabled _barrier "QueryAndPhysics")
  (Rendering|Material|SetMaterial _barrier 0 "/Game/Dynamic/Terrain/Red_Barrier.Red_Barrier"))